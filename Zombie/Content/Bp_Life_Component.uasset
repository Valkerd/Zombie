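; Life component that stores an actor's integer Hp against HpMax.
; BeginPlay clamps Hp between zero and HpMax, while LoseGainLife subtracts the passed amount without re-clamping, so negative amounts add life.
; GetHealthPercent divides Hp by HpMax before converting to double, so integer division drops the fractional part.
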(event EventBeginPlay
  (Variables|Default|SetHp (Math|Integer|Clamp(Integer) (Variables|Default|GetHp) 0 (Variables|Default|GetHpMax))))

(event EventTick
  (params (DeltaSeconds :type Float%20%28single-precision%29)))

(fn LoseGainLife
  (params (HptoLose :type Integer))
  (Variables|Default|SetHp (- (Variables|Default|GetHp) HptoLose))
  (return))

(fn GetHealthPercent
  (return (Math|Conversions|ToFloat(Integer) (/ (Variables|Default|GetHp) (Variables|Default|GetHpMax)))))